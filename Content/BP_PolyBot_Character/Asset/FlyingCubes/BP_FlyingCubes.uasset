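; Flying cube actor that drifts up and down along the Z axis, part of the PolyBot character assets.
; BeginPlay stores the start location and randomly flips the initial direction.
; Each Tick moves the actor by MovementSpeed with a random per-frame multiplier, giving uneven motion.
; Once it travels past MaxDistance, it reverses and takes its current position as the new start point.
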(event Custom|Movement
  (params (Delta%20Seconds :type Float%20%28double-precision%29))
  (bind _output_get (Variables|Default|SetCurrentLocation (+ (* Delta%20Seconds (Math|Vector|MakeVector 0.0 0.0 (* (Variables|Default|GetMovementSpeed) (Math|Random|RandomFloatinRange 1.0 6.0)))) (.location (Transformation|GetActorTransform (Components|GetOwner (Variables|Default|GetCube)))))))
  (Transformation|SetActorLocation (Components|GetOwner (Variables|Default|GetCube)) _output_get false false))

(event EventBeginPlay
  (Variables|Default|SetStartLocation (Transformation|GetActorLocation (Components|GetOwner (Variables|Default|GetCube))))
  (if (Math|Random|RandomBool)
    (Variables|Default|SetMovementSpeed (* (Variables|Default|GetMovementSpeed) -1.0))))

(event Collision|EventActorBeginOverlap
  (params (OtherActor :type Actor%20Object%20Reference)))

(event EventTick
  (params (DeltaSeconds :type Float%20%28single-precision%29))
  (bind _output_get (Variables|Default|SetDelta%20Seconds DeltaSeconds))
  (CallFunction|Movement _output_get)
  (if (> (Math|Vector|Distance(Vector) (Variables|Default|GetStartLocation) (Variables|Default|GetCurrentLocation)) (Variables|Default|GetMaxDistance))
    (Variables|Default|SetStartLocation (.location (Transformation|GetActorTransform (Components|GetOwner (Variables|Default|GetCube)))))
    (Variables|Default|SetMovementSpeed (* (Variables|Default|GetMovementSpeed) -1.0))))

(fn ConstructionScript)

(fn OnRepCurrentLocation)

(fn OnRepMaxDistance)